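; BP_Trap is a fire trap that repeatedly applies a Gameplay Effect to players standing inside its Box.
; On the server, overlaps add and remove each BP_Player's Ability System Component in a tracked list.
; A looping timer applies one shared effect spec, rebuilt from the latest entrant, to every tracked component.
; The timer starts on entry if inactive and clears when the list empties.
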(event OnComponentBeginOverlap(Box)
  (params (OverlappedComponent :type Primitive%20Component%20Object%20Reference) (OtherActor :type Actor%20Object%20Reference) (OtherComp :type Primitive%20Component%20Object%20Reference) (OtherBodyIndex :type Integer) (bFromSweep :type Boolean) (SweepResult :type Hit%20Result%20Structure%20%28by%20ref%29))
  (Networking|SwitchHasAuthority
    (:Authority
      (bind _asbp_player (Utilities|Casting|CastToBP_Player OtherActor))
      (Utilities|Array|Add (Variables|Default|GetASCompOnTrap) (Ability|GetAbilitySystemComponent _asbp_player))
      (Variables|Default|SetgameplayEffectSpec (GameplayEffects|MakeOutgoingSpec (Ability|GetAbilitySystemComponent _asbp_player) (Variables|Default|GetGameplayEffectClass) 0.0 (GameplayEffects|MakeEffectContext (Ability|GetAbilitySystemComponent _asbp_player))))
      (if (not (Utilities|Time|IsTimerActivebyHandle (Variables|Default|GettimerHandle)))
        (bind _returnvalue (Utilities|Time|SetTimerbyEvent (EventDispatchers|CreateEvent :!event Custom|OnTrapEffect_Event) 0.2 true))
        (Variables|Default|SettimerHandle _returnvalue)))))

(event OnComponentEndOverlap(Box)
  (params (OverlappedComponent :type Primitive%20Component%20Object%20Reference) (OtherActor :type Actor%20Object%20Reference) (OtherComp :type Primitive%20Component%20Object%20Reference) (OtherBodyIndex :type Integer))
  (Networking|SwitchHasAuthority
    (:Authority
      (bind _asbp_player (Utilities|Casting|CastToBP_Player OtherActor))
      (Utilities|Array|RemoveItem (Variables|Default|GetASCompOnTrap) (Ability|GetAbilitySystemComponent _asbp_player))
      (if (<= (Utilities|Array|Length (Variables|Default|GetASCompOnTrap)) 0)
        (Utilities|Time|ClearandInvalidateTimerbyHandle (Variables|Default|GettimerHandle))))))

(event Custom|OnTrapEffect_Event
  (for _array_element (Variables|Default|GetASCompOnTrap)
    (GameplayEffects|ApplyGameplayEffectSpecToTarget _array_element (Variables|Default|GetgameplayEffectSpec) _array_element)))

(event EventBeginPlay)

(event Collision|EventActorBeginOverlap
  (params (OtherActor :type Actor%20Object%20Reference)))

(event EventTick
  (params (DeltaSeconds :type Float%20%28single-precision%29)))

(fn ConstructionScript)