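; BP_EffectActor is a world actor that applies a configurable Gameplay Effect to a BP_Player that overlaps it.
; The ApplicationPolicy setting selects whether ApplyEffectToTarget fires when the overlap begins, when it ends, or both.
; The Construction Script writes the effect class's display name to a TextRender component whenever a valid class is set, labeling each placed instance.
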(event EventBeginPlay)

(event Collision|EventActorBeginOverlap
  (params (OtherActor :type Actor%20Object%20Reference))
  (bind _asbp_player (Utilities|Casting|CastToBP_Player OtherActor))
  (switch Utilities|FlowControl|Switch|SwitchonEEffectApplicationPolicy (Variables|Default|GetApplicationPolicy)
    (:ApplyOnOverlap
      _)
    (:ApplyOnBoth
      _))
  (Class|ARPGEffectActor|ApplyEffecttoTarget _asbp_player (Variables|Default|GetGameplayEffectClass)))

(event Collision|EventActorEndOverlap
  (params (OtherActor :type Actor%20Object%20Reference))
  (bind _asbp_player (Utilities|Casting|CastToBP_Player OtherActor))
  (switch Utilities|FlowControl|Switch|SwitchonEEffectApplicationPolicy (Variables|Default|GetApplicationPolicy)
    (:ApplyOnEndOverlap
      _)
    (:ApplyOnBoth
      _))
  (Class|ARPGEffectActor|ApplyEffecttoTarget _asbp_player (Variables|Default|GetGameplayEffectClass)))

(fn ConstructionScript
  (bind _gameplayeffectclass (Variables|Default|GetGameplayEffectClass))
  (if (Utilities|IsValidClass _gameplayeffectclass)
    (Rendering|Components|TextRender|SetText (Variables|Default|GetTextRender) (Utilities|Text|ToText(String) (Utilities|GetClassDisplayName _gameplayeffectclass)))))